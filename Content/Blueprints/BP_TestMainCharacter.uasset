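; BP_TestMainCharacter is a test player character that moves from input axes and tracks its distance to an anchor point.
; Forward_Backward moves along the actor's forward vector, while Left_Right both strafes and turns the controller yaw.
; BeginPlay caches the X position of BP_AnchorPoint and the starting X offset as MaxDistance, which is not read here.
; Tick recomputes the signed X-only distance to that cached target and prints it.
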(event EventBeginPlay
  ;[1 1 1] Get location of the target at the begining
  (bind _returnvalue (Actor|GetActorOfClass "/Game/Blueprints/BP_AnchorPoint.BP_AnchorPoint_C"))
  (bind _output_get (Variables|Default|SetTarget (.x (Transformation|GetActorLocation _returnvalue))))
  (Variables|Default|SetMaxDistance (- _output_get (.x (Transformation|GetActorLocation)))))

(event EventTick
  (params (DeltaSeconds :type Float%20%28single-precision%29))
  ;[1 1 1] Set the distance between the actor and the target each tick
  (bind _output_get (Variables|Default|SetDistance (- (Variables|Default|GetTarget) (.x (Transformation|GetActorLocation)))))
  (Development|PrintString (Utilities|String|ToString(Float) _output_get)))

(event Input|AxisEvents|InputAxisForward_Backward
  (params (AxisValue :type Float%20%28single-precision%29))
  ;[1 1 1] Movement player
  (Pawn|Input|AddMovementInput (Transformation|GetActorForwardVector) AxisValue false))

(event Input|AxisEvents|InputAxisLeft_Right
  (params (AxisValue :type Float%20%28single-precision%29))
  ;[1 1 1] Movement player
  (Pawn|Input|AddMovementInput (Transformation|GetActorRightVector) AxisValue false)
  (Pawn|Input|AddControllerYawInput AxisValue))

(fn ConstructionScript)