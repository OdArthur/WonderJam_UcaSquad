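; Player character with axis movement (strafing also turns the view), a pause menu, and a darkness threat outside torch range.
; Leaving a BP_Torch overlap plays a dark sound, enables post-process, and tightens material parameter collection values through delayed stages, ending in a placeholder "DED" print.
; Re-entering a torch fades the sound, restores the visuals and zeroes TimeNotInRange, a stage counter that pending delays check before advancing.
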(event OnComponentEndOverlap(CapsuleComponent)
  (params (OverlappedComponent :type Primitive%20Component%20Object%20Reference) (OtherActor :type Actor%20Object%20Reference) (OtherComp :type Primitive%20Component%20Object%20Reference) (OtherBodyIndex :type Integer))
  (Utilities|Casting|CastToBP_Torch OtherActor)
  ;[1 1 1] Audio fx
  (bind _returnvalue (Audio|SpawnSound2D "/Game/Audio/DarkSound.DarkSound" 1.0 1.0 0.0 0))
  (Components|Activation|SetActive _returnvalue false false)
  (Components|Activation|ToggleActive _returnvalue)
  (bind _output_get (Variables|Default|SetTimeNotInRange 1))
  (Variables|/Script/Engine.PostProcessComponent|SetbEnabled (Variables|Default|GetPostProcess) true)
  (if (> _output_get 0)
    (Variables|Default|SetTimeNotInRange 11)
    (Utilities|FlowControl|Delay 1e+01)
    (if (> (Variables|Default|GetTimeNotInRange) 10)
      (Rendering|Material|SetScalarParameterValue "/Game/PostProcess/paramColl.paramColl" "Radius_max" 1.0 :!class /Script/Engine.KismetMaterialLibrary)
      (Rendering|Material|SetScalarParameterValue "/Game/PostProcess/paramColl.paramColl" "Radius_min" 0.45 :!class /Script/Engine.KismetMaterialLibrary)
      (Rendering|Material|SetScalarParameterValue "/Game/PostProcess/paramColl.paramColl" "Density" 1e+01 :!class /Script/Engine.KismetMaterialLibrary)
      (Variables|Default|SetTimeNotInRange 21)
      (if (> (Variables|Default|GetTimeNotInRange) 20)
        (Utilities|FlowControl|Delay 1e+01)
        (if (> (Variables|Default|GetTimeNotInRange) 20)
          (Rendering|Material|SetScalarParameterValue "/Game/PostProcess/paramColl.paramColl" "Radius_max" 1.0 :!class /Script/Engine.KismetMaterialLibrary)
          (Rendering|Material|SetScalarParameterValue "/Game/PostProcess/paramColl.paramColl" "Radius_min" 0.2 :!class /Script/Engine.KismetMaterialLibrary)
          (Rendering|Material|SetScalarParameterValue "/Game/PostProcess/paramColl.paramColl" "Density" 2.0 :!class /Script/Engine.KismetMaterialLibrary)
          (if (> (Variables|Default|GetTimeNotInRange) 20)
            (Variables|Default|SetTimeNotInRange 31)
            (Utilities|FlowControl|Delay 1e+01)
            (if (> (Variables|Default|GetTimeNotInRange) 30)
              (Development|PrintString "DED"))))))))

(event OnComponentBeginOverlap(CapsuleComponent)
  (params (OverlappedComponent :type Primitive%20Component%20Object%20Reference) (OtherActor :type Actor%20Object%20Reference) (OtherComp :type Primitive%20Component%20Object%20Reference) (OtherBodyIndex :type Integer) (bFromSweep :type Boolean) (SweepResult :type Hit%20Result%20Structure%20%28by%20ref%29))
  (Utilities|Casting|CastToBP_Torch OtherActor)
  ;[1 1 1] Audio fx
  (Utilities|IsValid (stale OnComponentEndOverlap(CapsuleComponent) _returnvalue)
    (:Is%20Valid
      (Audio|Components|Audio|FadeOut (stale OnComponentEndOverlap(CapsuleComponent) _returnvalue) 1.0 0.0 "Linear" :!class /Script/Engine.AudioComponent)
      (Variables|Default|SetTimeNotInRange (- (Variables|Default|GetTimeNotInRange) (Variables|Default|GetTimeNotInRange)))
      (Variables|/Script/Engine.PostProcessComponent|SetbEnabled (Variables|Default|GetPostProcess) false)
      (Rendering|Material|SetScalarParameterValue "/Game/PostProcess/paramColl.paramColl" "Radius_max" 2.0 :!class /Script/Engine.KismetMaterialLibrary)
      (Rendering|Material|SetScalarParameterValue "/Game/PostProcess/paramColl.paramColl" "Radius_min" 0.6 :!class /Script/Engine.KismetMaterialLibrary)
      (Rendering|Material|SetScalarParameterValue "/Game/PostProcess/paramColl.paramColl" "Density" 3e+01 :!class /Script/Engine.KismetMaterialLibrary))
    (:Is%20Not%20Valid
      (Development|PrintString "Cant load fx ombre de la mort sound in BP_Player"))))

(event Input|ActionEvents|InputActionPauseInput
  (params (Key :type Key%20Structure :default "None"))
  (:Pressed
    (Game|SetGamePaused true)
    (bind _returnvalue (UserInterface|CreateWidget "/Game/UI/W_Pause.W_Pause_C"))
    (UserInterface|Viewport|AddtoViewport _returnvalue 0)))

(event Input|AxisEvents|InputAxisForward_Backward
  (params (AxisValue :type Float%20%28single-precision%29))
  ;[1 1 1] Movement player
  (Pawn|Input|AddMovementInput (Transformation|GetActorForwardVector) AxisValue false))

(event Input|AxisEvents|InputAxisLeft_Right
  (params (AxisValue :type Float%20%28single-precision%29))
  ;[1 1 1] Movement player
  (Pawn|Input|AddMovementInput (Transformation|GetActorRightVector) AxisValue false)
  (Pawn|Input|AddControllerYawInput AxisValue))

(fn ConstructionScript)