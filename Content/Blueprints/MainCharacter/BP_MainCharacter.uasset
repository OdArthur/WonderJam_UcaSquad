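; Main character Blueprint that decides win or loss from keys missed along a patrol path.
; BeginPlay measures the path's X span, and Tick compares the character's X distance from its start against five evenly spaced checkpoints.
; Passing one destroys any remaining collectible there and counts a miss, while PlayerPickedAKey just advances the key index.
; At index five, three or more misses open the lose menu, otherwise the win menu.
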(event Custom|PlayerPickedAKey
  ;[1 1 1] For when player get a key
  (Variables|Default|SetKeyIndex (+ (Variables|Default|GetKeyIndex) 1)))

(event EventBeginPlay
  (bind _patrolpath (Variables|Default|GetPatrolPath))
  (bind _returnvalue (Transformation|GetActorLocation _patrolpath))
  (bind _patrolpoints (Variables|/Game/Blueprints/MainCharacter/BP_PatrolPath.BP_PatrolPath_C|GetPatrolPoints _patrolpath))
  (bind _output (Utilities|Array|Get(acopy) _patrolpoints))
  (bind _returnvalue_2 (+ (.x _output) (.x _returnvalue)))
  ;[1 1 1] Get location of the target at the begining
  (Variables|Default|SetStart _returnvalue_2)
  (Variables|Default|SetMaxDistance (Math|Float|Absolute(Float) (- (+ (.x (Utilities|Array|Get(acopy) _patrolpoints (Utilities|Array|LastIndex _patrolpoints))) (.x _returnvalue)) _returnvalue_2))))

(event EventTick
  (params (DeltaSeconds :type Float%20%28single-precision%29))
  ;[1 1 1] Set the distance between the actor and the target each tick
  (Variables|Default|SetDistance (Math|Float|Absolute(Float) (- (Variables|Default|GetStart) (.x (Transformation|GetActorLocation)))))
  ;[1 1 1] Delete Key if checkpoint passed
  (if (== (Variables|Default|GetKeyIndex) 5)
    (if (>= (Variables|Default|GetKeyCounter) 3)
      (Game|OpenLevel(byObjectReference) "/Game/Maps/LoseMenu.LoseMenu")
      (else
        (Game|OpenLevel(byObjectReference) "/Game/Maps/WinMenu.WinMenu")))
    (elif (>= (Variables|Default|GetDistance) (* (/ (Variables|Default|GetMaxDistance) 5.0) (+ (Variables|Default|GetKeyIndex) 1)))
      (Utilities|IsValid (Utilities|Array|Get(acopy) (Variables|Default|GetCollectibles) (Variables|Default|GetKeyIndex))
        (:Is%20Valid
          (Actor|DestroyActor (Utilities|Array|Get(acopy) (Variables|Default|GetCollectibles) (Variables|Default|GetKeyIndex)))
          (Variables|Default|SetKeyIndex (+ (Variables|Default|GetKeyIndex) 1))
          (Variables|Default|SetKeyCounter (+ (Variables|Default|GetKeyCounter) 1)))
        (:Is%20Not%20Valid
          (Variables|Default|SetKeyIndex (+ (Variables|Default|GetKeyIndex) 1)))))))

(fn ConstructionScript)