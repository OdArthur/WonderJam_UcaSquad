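; BP_CollectibleKey is a key pickup that raises the player's key count when collected.
; Each tick it spins the key mesh and bobs it vertically, using a cosine of an incrementing per-frame counter.
; A sphere overlap plays the pickup sound at world origin before casting the overlapping actor's instigator to BP_Player.
; On a successful cast it increments KeyCounter and destroys itself.
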(event OnComponentBeginOverlap(SphereCollisionRadius)
  (params (OverlappedComponent :type Primitive%20Component%20Object%20Reference) (OtherActor :type Actor%20Object%20Reference) (OtherComp :type Primitive%20Component%20Object%20Reference) (OtherBodyIndex :type Integer) (bFromSweep :type Boolean) (SweepResult :type Hit%20Result%20Structure%20%28by%20ref%29))
  (Audio|PlaySoundatLocation "/Game/Audio/picking-up-keys-from-floor.picking-up-keys-from-floor" "0, 0, 0" "0, 0, 0" 1.0 1.0 0.0 0 0 0 0)
  (bind _asbp_player (Utilities|Casting|CastToBP_Player (Game|GetInstigator OtherActor)))
  (Math|Integer|IncrementInt (Variables|/Game/Blueprints/BP_Player.BP_Player_C|GetKeyCounter _asbp_player)
    (:%20%20
      (Actor|DestroyActor))))

(event EventTick
  (params (DeltaSeconds :type Float%20%28single-precision%29))
  (bind _worn_key (Variables|Default|GetWorn_Key))
  (Transformation|AddRelativeRotation _worn_key (Math|Rotator|MakeRotator 0.0 0.0 (Math|Conversions|ToFloat(Integer) (Variables|Default|GetSpeedRotation))) false false)
  (bind _result (Math|Float|IncrementFloat (Variables|Default|GetTimeMovement))
    (:%20%20
      (Transformation|AddRelativeLocation _worn_key (Math|Vector|MakeVector 0.0 0.0 (/ (Math|Trig|Cos(Degrees) _result) 2.0)) false false))))

(fn ConstructionScript)